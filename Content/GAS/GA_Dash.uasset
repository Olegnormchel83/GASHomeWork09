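; Gameplay ability that instantly dashes the avatar forward by a default distance, with a particle burst and teleport sound at the starting point.
; An object line trace along the forward vector shortens the dash using the hit location's distance, without checking whether anything was hit.
; A swept SetActorLocation performs the move, then the ability ends, or cancels upfront if the avatar is invalid.
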(event Ability|EventActivateAbility
  (bind _returnvalue (Ability|GetAvatarActorfromActorInfo))
  (bind _defaultdashdistance (Variables|Default|GetDefaultDashDistance))
  (Utilities|IsValid _returnvalue
    (:Is%20Valid
      (Variables|Default|SetDashDistance (Variables|Default|GetDefaultDashDistance))
      (bind _output_get (Variables|Default|SetAvatarActor _returnvalue))
      (Effects|SpawnEmitteratLocation "/Game/FXVarietyPack/Particles/P_ky_hit1.P_ky_hit1" (Transformation|GetActorLocation _output_get) (Transformation|GetActorRotation _output_get) "0.600000,0.600000,0.600000")
      (Audio|PlaySoundatLocation "/Engine/VREditor/Sounds/VR_teleport_Cue.VR_teleport_Cue" (Transformation|GetActorLocation _output_get) "0, 0, 0" 0.5 1.0 0.0 0 0 0 0)
      (bind _outhit (Collision|LineTraceForObjects (Transformation|GetActorLocation _output_get) (+ (Transformation|GetActorLocation _output_get) (* (Transformation|GetActorForwardVector _output_get) (Variables|Default|GetDefaultDashDistance))) (Utilities|Array|MakeArray "ObjectTypeQuery1" "ObjectTypeQuery2" "ObjectTypeQuery4") false 0 "None"))
      (if (< (Math|Vector|Distance(Vector) (.Location (Collision|BreakHitResult _outhit)) (Transformation|GetActorLocation (Variables|Default|GetAvatarActor))) _defaultdashdistance)
        (Variables|Default|SetDashDistance (Math|Float|Clamp(Float) (Math|Vector|Distance(Vector) (.Location (Collision|BreakHitResult _outhit)) (Transformation|GetActorLocation (Variables|Default|GetAvatarActor))) 0.0 _defaultdashdistance)))
      (Transformation|SetActorLocation (Variables|Default|GetAvatarActor) (+ (Transformation|GetActorLocation (Variables|Default|GetAvatarActor)) (* (Transformation|GetActorForwardVector (Variables|Default|GetAvatarActor)) (Variables|Default|GetDashDistance))) true false)
      (Ability|EndAbility))
    (:Is%20Not%20Valid
      (Ability|CancelAbility))))

(event Ability|EventOnEndAbility
  (params (bWasCancelled :type Boolean)))